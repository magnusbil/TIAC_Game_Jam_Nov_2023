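; Turtle enemy that wanders the level and hides when Cuthbert_BP, likely the player, comes near.
; On BeginPlay it loops AI MoveTo to random reachable points around itself, pausing briefly after each successful move.
; Overlap on HideBox sets Hiding and stops the AI controller's movement through a DoOnce.
; When Cuthbert_BP leaves the box, it clears Hiding, resumes wandering after a short delay, then resets the DoOnce.
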(event `self.ReceiveBeginPlay`
  (`self.Wander`))

(event `Wander`
  (if (not (`self.Hiding`))
    (`|AIMoveTo` (`AIBlueprintHelperLibrary.GetAIController` self) null (`NavigationSystemV1.K2_GetRandomReachablePointInRadius` (`self.K2_GetActorLocation`) 1000.0 null null) null
      (:`OnSuccess`
        (`KismetSystemLibrary.Delay` (`KismetMathLibrary.RandomFloatInRange` 0.2 0.6))
        (`self.Wander`)))))

(event `self.HideBox.OnComponentBeginOverlap`
  (params (OverlappedComponent :type "PrimitiveComponent Object Reference") (OtherActor :type "Actor Object Reference") (OtherComp :type "PrimitiveComponent Object Reference") (OtherBodyIndex :type Integer) (bFromSweep :type Boolean) (SweepResult :type "HitResult Structure (by ref)"))
  (if (== (`GameplayStatics.GetObjectClass` OtherActor) "/Game/Blueprint/Character/Cuthbert_BP.Cuthbert_BP_C")
    (`/Engine/EditorBlueprintResources/StandardMacros.DoOnce` false :!label _label
      (:`Completed`
        (set `self.Hiding` true)
        (`Controller.StopMovement` (`AIBlueprintHelperLibrary.GetAIController` self))))))

(event `self.HideBox.OnComponentEndOverlap`
  (params (OverlappedComponent :type "PrimitiveComponent Object Reference") (OtherActor :type "Actor Object Reference") (OtherComp :type "PrimitiveComponent Object Reference") (OtherBodyIndex :type Integer))
  (if (== (`GameplayStatics.GetObjectClass` OtherActor) "/Game/Blueprint/Character/Cuthbert_BP.Cuthbert_BP_C")
    (set `self.Hiding` false)
    (`KismetSystemLibrary.Delay` 0.2)
    (`self.Wander`)
    (goto _label :!via `Reset`)))

(fn `UserConstructionScript`)