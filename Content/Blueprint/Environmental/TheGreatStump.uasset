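; The Great Stump is an environmental actor that trades a marble check for a sword when the player overlaps it.
; On overlap it looks up each NecessaryMarbles entry in Cuthbert's inventory item names, stopping at the first one missing.
; The success test compares the index to Min(length, 1) rather than the last index, so matching the first two marbles suffices.
; It then spawns the Sword beside the player and destroys itself.
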(event `self.ReceiveActorBeginOverlap`
  (params (OtherActor :type "Actor Object Reference"))
  (bind _returnvalue (`GameplayStatics.GetPlayerCharacter` 0))
  (bind _returnvalue_2 (`self.GetTransform` (`GameplayStatics.GetPlayerCharacter` 0)))
  (if (== OtherActor _returnvalue)
    (bind _ascuthbert_bp (cast `/Game/Blueprint/Character/Cuthbert_BP` _returnvalue))
    (for (_array_element _array_index) (`self.NecessaryMarbles`)
      (if (`KismetArrayLibrary.Array_Contains` (`/Game/Blueprint/Inventory/W_Inventory.ItemNames` (`/Game/Blueprint/Character/Cuthbert_BP.Inventory` _ascuthbert_bp)) _array_element)
        (`KismetSystemLibrary.PrintString` (`KismetStringLibrary.Conv_IntToString` _array_index))
        (if (== _array_index (`KismetMathLibrary.Min` (`KismetArrayLibrary.Array_Length` (`self.NecessaryMarbles`)) 1))
          (`|SpawnActorFromClass` "/Game/Blueprint/Items/Sword.Sword_C" (`KismetMathLibrary.MakeTransform` (`KismetMathLibrary.MakeVector` (+ (.x (.location _returnvalue_2)) -15.0) (+ (.y (.location _returnvalue_2)) 100.0) (.z (.location _returnvalue_2)))) "AlwaysSpawn" "MultiplyWithRoot" null null)
          (`self.K2_DestroyActor`))
        (else
          (break))))))

(fn `UserConstructionScript`)