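; StumpWithSword is an environment actor that gives way to a Sword once the player holds the right marbles.
; On player overlap, it loops MarblesNeeded against Cuthbert_BP's MarblesCollected.
; The spawn fires on a match at index Min(length, 1), so only the second entry effectively gates it, not the whole list.
; It spawns the Sword at a fixed offset from the player, then destroys itself.
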(event `self.ReceiveActorBeginOverlap`
  (params (OtherActor :type "Actor Object Reference"))
  (bind _marblesneeded (`self.MarblesNeeded`))
  (bind _returnvalue (`self.GetTransform` (`GameplayStatics.GetPlayerCharacter` 0)))
  (if (== OtherActor (`GameplayStatics.GetPlayerCharacter` 0))
    (bind _ascuthbert_bp (cast `/Game/Blueprint/Character/Cuthbert_BP` OtherActor))
    (for (_array_element _array_index) _marblesneeded
      (if (`KismetArrayLibrary.Array_Contains` (`/Game/Blueprint/Character/Cuthbert_BP.MarblesCollected` _ascuthbert_bp) _array_element)
        (if (== (`KismetMathLibrary.Min` (`KismetArrayLibrary.Array_Length` _marblesneeded) 1) _array_index)
          (`|SpawnActorFromClass` "/Game/Blueprint/Items/Sword.Sword_C" (`KismetMathLibrary.MakeTransform` (`KismetMathLibrary.MakeVector` (+ (.x (.location _returnvalue)) -15.0) (+ (.y (.location _returnvalue)) 20.0) (.z (.location _returnvalue)))) "Undefined" "MultiplyWithRoot" null null)
          (`self.K2_DestroyActor`))))))

(fn `UserConstructionScript`)